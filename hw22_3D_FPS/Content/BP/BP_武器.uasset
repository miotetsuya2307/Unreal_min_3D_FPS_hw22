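; BP_武器 is a weapon Blueprint with automatic fire and magazine-based ammo.
; Holding the 開槍 input runs a Delay loop that spawns BP_子彈 at the muzzle socket, passes it the weapon damage, plays a small explosion effect and spends a round.
; Event 換彈匣 refills the magazine from reserve ammo, limited to what remains.
; Event 補充子彈 adds one magazine's worth to the reserve, clamped to its maximum.
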(event `InputAction|開槍`
  (params (Key :type "Key Structure"))
  (bind `_武器` (`self.武器`))
  ;[1 1 1] 開槍
  (:`Pressed`
    (set `self.開槍中` true)
    (if (and (> (`self.目前子彈數量`) 0) (`self.開槍中`)) :!label _label
      (bind _returnvalue (`|SpawnActorFromClass` "/Game/BP/BP_子彈.BP_子彈_C" (`SceneComponent.GetSocketTransform` (`self.武器`) "子彈插槽" "RTS_World") "Undefined" "OverrideRootScale" null null)) ; 生成子彈藍圖
      (set `/Game/BP/BP_子彈.目前武器傷害` (`self.武器傷害`) _returnvalue) ; 將武器傷害傳給子彈
      (`GameplayStatics.SpawnEmitterAtLocation` "/Game/StarterContent/Particles/P_Explosion.P_Explosion" (`SceneComponent.GetSocketLocation` `_武器` "子彈插槽") (`SceneComponent.GetSocketRotation` `_武器` "None") (0.1 0.1 0.1))
      (set `self.目前子彈數量` (- (`self.目前子彈數量`) 1))
      (`KismetSystemLibrary.Delay` (`self.開槍間隔`))
      (goto _label)))
  (:`Released`
    (set `self.開槍中` false)))

(event `換彈匣`
  ;[0.1333 1 0.2902] 計算要補充裝幾顆子彈
  (set `self.要補充的子彈數量` (- (`self.彈匣尺寸`) (`self.目前子彈數量`))) ; 計算要補充的子彈數量
  ;[0.1333 1 0.2902] 判斷總數是否>=要補充的數量
  (if (not (>= (`self.子彈總數`) (`self.要補充的子彈數量`)))
    ;[0.1333 1 0.2902] 總數<=要補充的數量
    (set `self.要補充的子彈數量` (`self.子彈總數`)))
  ;[0.1333 1 0.2902] 目前子彈以及總數更新
  (set `self.目前子彈數量` (+ (`self.目前子彈數量`) (`self.要補充的子彈數量`))) ; 補充子彈數量
  (set `self.子彈總數` (- (`self.子彈總數`) (`self.要補充的子彈數量`))) ; 扣除子彈總數
)

(event `補充子彈`
  ;[0.1333 1 0.2902] 補充子彈
  (bind _output_get (set `self.子彈總數` (+ (`self.子彈總數`) (`self.彈匣尺寸`)))) ; 子彈總數+彈匣尺寸
  (set `self.子彈總數` (`KismetMathLibrary.Clamp` _output_get 0 (`self.子彈上限`))))

(fn `UserConstructionScript`)