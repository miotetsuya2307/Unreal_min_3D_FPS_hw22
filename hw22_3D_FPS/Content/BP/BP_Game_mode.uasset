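; Game mode Blueprint that runs a minute-and-second countdown and records how many sea monsters must be killed.
; Tick feeds a one-second Delay, which throttles the decrement, rolls seconds over into minutes, and pauses the game when time runs out.
; BeginPlay counts actors tagged Sea_monster and stores that as the required kill count, which this graph does not otherwise use.
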(event `self.ReceiveTick`
  (params (DeltaSeconds :type "Float (single-precision)"))
  ;[0.1022 0.3885 0.08518] 倒數系統
  ;;[1 1 1] 每秒秒數減一
  (`KismetSystemLibrary.Delay` 1.0) ; 延遲
  (bind _output_get (set `self.秒` (- (`self.秒`) 1)))
  ;;[1 1 1] 當s為0，s設為59
  (if (< _output_get 0)
    (set `self.秒` 59)
    ;;[1 1 1] 當m>0，m-1
    (if (> (`self.分`) 0)
      (set `self.分` (- (`self.分`) 1))
      (else
        ;;[1 1 1] 當m為0；s=59時，s設為0，結束遊戲
        (if (== (`self.秒`) 59)
          (set `self.秒` 0)
          (`GameplayStatics.SetGamePaused` true))))))

(event `self.ReceiveBeginPlay`
  ;[0.03724 0.176 0.1535] 取得貼有Sea_monster標籤的所有物件，
  ; 並儲存數量
  (bind _outactors (`GameplayStatics.GetAllActorsWithTag` "Sea_monster"))
  (set `self.需要擊殺的怪物數量` (`KismetArrayLibrary.Array_Length` _outactors)))

(fn `UserConstructionScript`)